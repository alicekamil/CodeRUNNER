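; BP_SpawnerFloor is a child spawner that builds and recycles floor tiles to form an endless road along the X axis.
; BeginPlay places the first tile at the spawner, measures its X bounds, then chains the remaining tiles end to end while tracking the rear one.
; When a tile hits bounds, it moves behind the rear tile after a tiny delay and becomes the new rear, avoiding respawns.
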(event `self.ReceiveBeginPlay`
  (bind (_returnvalue_x _returnvalue_y) (`KismetMathLibrary.BreakVector` (`self.K2_GetActorLocation` (`self.RearTile`))))
  (`parent.ReceiveBeginPlay`)
  (for _index (range (+ (`self.ActorsRequiredCount`) 1))
    (if (== _index 0)
      ;[1 1 1] If first floor tile
      (bind _returnvalue (`self.SpawnActor`))
      (set `self.RearTile` _returnvalue)
      (set `self.TileSize` (* (.x (`.BoxExtent` (`self.GetActorBounds` _returnvalue false false))) 2.0))
      (`self.K2_SetActorLocation` (`self.RearTile`) (`self.K2_GetActorLocation`) false false)
      (else
        ;[1 1 1] If not first tile
        (bind _returnvalue_2 (`self.SpawnActor`))
        (`self.K2_SetActorLocation` _returnvalue_2 (`KismetMathLibrary.MakeVector` (+ _returnvalue_x (`self.TileSize`)) _returnvalue_y) false false)
        (set `self.RearTile` _returnvalue_2)))))

(event `self.SpawnActorHitBounds`
  (params (OutOfBoundsActor :type "Actor Object Reference"))
  (bind (_returnvalue_x _returnvalue_y _returnvalue_z) (`KismetMathLibrary.BreakVector` (`self.K2_GetActorLocation` (`self.RearTile`))))
  ;[1 1 1] When a tile gets out of bound, its gonna find the rear tile(end of road), find its location, add tile size of the offset against it and move it back that distance and make it the current rear tile
  (`KismetSystemLibrary.Delay` 0.01)
  (`self.K2_SetActorLocation` OutOfBoundsActor (`KismetMathLibrary.MakeVector` (+ _returnvalue_x (`self.TileSize`)) _returnvalue_y _returnvalue_z) false false)
  (set `self.RearTile` OutOfBoundsActor))

(fn `SpawnActor`
  (returns (ReturnValue :type "Actor Object Reference"))
  (bind _returnvalue (`parent.SpawnActor`))
  (return _returnvalue))

(fn `UserConstructionScript`
  (`parent.UserConstructionScript`))